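; EnemyRangerBullet is an enemy ranged projectile that damages the player's TopDownCharacter on overlap.
; On BeginPlay a one-shot timer destroys it once its LifeTime runs out.
; Overlapping an actor whose class is exactly TopDownCharacter applies AttackDamage and destroys the bullet, while other overlaps are ignored.
; The graphs contain no movement logic.
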(event `self.ReceiveBeginPlay`
  (`KismetSystemLibrary.K2_SetTimerDelegate` (delegate `DestroyByOldAge`) (`self.LifeTime`)))

(event `DestroyByOldAge`
  (`self.K2_DestroyActor`))

(event `self.ReceiveTick`
  (params (DeltaSeconds :type "Float (single-precision)")))

(event `self.ReceiveActorBeginOverlap`
  (params (OtherActor :type "Actor Object Reference"))
  (if (== (`GameplayStatics.GetObjectClass` OtherActor) "/Game/TopDownBP/Blueprints/TopDownCharacter.TopDownCharacter_C")
    (`GameplayStatics.ApplyDamage` OtherActor (`self.AttackDamage`))
    (`self.K2_DestroyActor`)))

(fn `UserConstructionScript`)