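; PlayerAttackBox is a short-lived player attack volume that damages all AI characters overlapping it when its lifetime timer ends.
; Begin and end overlap events maintain the list of AI_Character targets.
; On expiry it clears DestroyAtDeath on each target's AIController1 and applies damage to that controller rather than the pawn.
; It then prints the hit count, calls DestroyCheck on every AIController1 and destroys itself.
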(event `self.ReceiveBeginPlay`
  ;[1 1 1] Set timer until dealing damage
  (`KismetSystemLibrary.K2_SetTimerDelegate` (delegate `DealDamage`) (`self.LifeTime`)))

(event `DealDamage`
  ;[1 1 1] Set timer until dealing damage
  ;[1 1 1] Deal damage if colliding, then destroy self
  (for _array_element (`self.CollidingEnemy`)
    (bind _returnvalue (`AIBlueprintHelperLibrary.GetAIController` _array_element))
    (bind _asaicontroller_1 (cast `/Game/AIController1` _returnvalue))
    (set `/Game/AIController1.DestroyAtDeath` false _asaicontroller_1)
    (`GameplayStatics.ApplyDamage` _returnvalue (`self.Damage`) null self "/Script/Engine.DamageType"))
  (`KismetSystemLibrary.PrintString` (`KismetStringLibrary.Concat_StrStr` "Hit " (`KismetStringLibrary.Conv_IntToString` (`KismetArrayLibrary.Array_Length` (`self.CollidingEnemy`))) " Enemies"))
  (bind _outactors (`GameplayStatics.GetAllActorsOfClass` "/Game/AIController1.AIController1_C"))
  (for _array_element_2 _outactors
    (bind _asaicontroller_1_2 (cast `/Game/AIController1` _array_element_2))
    (`/Game/AIController1.DestroyCheck` _asaicontroller_1_2))
  (`self.K2_DestroyActor`))

(event `self.ReceiveActorBeginOverlap`
  (params (OtherActor :type "Actor Object Reference"))
  ;[1 1 1] Colliding with enemy
  (if (== (`GameplayStatics.GetObjectClass` OtherActor) "/Game/AI_Character.AI_Character_C")
    (`KismetArrayLibrary.Array_AddUnique` (`self.CollidingEnemy`) OtherActor)))

(event `self.ReceiveActorEndOverlap`
  (params (OtherActor :type "Actor Object Reference"))
  ;[1 1 1] Stop colliding with enemy
  (`KismetArrayLibrary.Array_RemoveItem` (`self.CollidingEnemy`) OtherActor))

(event `self.ReceiveTick`
  (params (DeltaSeconds :type "Float (single-precision)")))

(fn `UserConstructionScript`)