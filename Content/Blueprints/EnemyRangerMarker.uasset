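; EnemyRangerMarker is a short-lived actor that fires a delayed ranged attack for an enemy ranger.
; On BeginPlay, a one-shot timer set to LifeTime spawns an EnemyRangerBullet slightly above and ahead of the marker, facing the same way.
; The bullet receives the marker's Damage and a fixed lifetime, then the marker destroys itself.
; If TheOwner is destroyed first, the marker destroys itself, cancelling the attack.
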(event `self.ReceiveBeginPlay`
  (`KismetSystemLibrary.K2_SetTimerDelegate` (delegate `Fire projectile`) (`self.LifeTime`)))

(event `Fire projectile`
  (bind _rotation (.rotation (`self.GetTransform`)))
  (`|SpawnActorFromClass` "/Game/Blueprints/EnemyRangerBullet.EnemyRangerBullet_C" (`KismetMathLibrary.MakeTransform` (+ (* (`KismetMathLibrary.GetUpVector` _rotation) 150.0) (* (`KismetMathLibrary.GetForwardVector` _rotation) 50.0) (.location (`self.GetTransform`))) _rotation (.scale (`self.GetTransform`))) "Undefined" "OverrideRootScale" null (`self.Damage`) 2.0)
  (`self.K2_DestroyActor`))

(event `self.ReceiveActorBeginOverlap`
  (params (OtherActor :type "Actor Object Reference")))

(event `self.ReceiveTick`
  (params (DeltaSeconds :type "Float (single-precision)")))

(event `self.TheOwner.OnDestroyed`
  ;[1 1 1] Cancel attack if owner gets killed.
  (`self.K2_DestroyActor`))

(fn `UserConstructionScript`)