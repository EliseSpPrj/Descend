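; EnemyAttackBox is a delayed-hit volume for enemy attacks that damages a TopDownCharacter caught inside it.
; Begin and end overlap events track a single TopDownCharacter reference, matched by exact class.
; A one-shot LifeTime timer applies damage to that character if still overlapping, then destroys the box.
; Destruction of the owner destroys the box early, cancelling the attack.
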(event `/Game/Blueprints/PlayerAttackBox.ReceiveBeginPlay`
  ;[1 1 1] Set timer until dealing damage
  (`KismetSystemLibrary.K2_SetTimerDelegate` (delegate `DealDamage`) (`self.LifeTime`)))

(event `DealDamage`
  (bind _collidingenemy (`self.CollidingEnemy`))
  ;[1 1 1] Set timer until dealing damage
  ;[1 1 1] Deal damage if colliding, then destroy self
  (if (== (`GameplayStatics.GetObjectClass` _collidingenemy) "/Game/TopDownBP/Blueprints/TopDownCharacter.TopDownCharacter_C")
    (`GameplayStatics.ApplyDamage` _collidingenemy (`self.Damage`) null self "/Script/Engine.DamageType"))
  (`self.K2_DestroyActor`))

(event `/Game/Blueprints/PlayerAttackBox.ReceiveActorBeginOverlap`
  (params (OtherActor :type "Actor Object Reference"))
  ;[1 1 1] Colliding with enemy
  (if (== (`GameplayStatics.GetObjectClass` OtherActor) "/Game/TopDownBP/Blueprints/TopDownCharacter.TopDownCharacter_C")
    (set `self.CollidingEnemy` OtherActor)))

(event `self.ReceiveActorEndOverlap`
  (params (OtherActor :type "Actor Object Reference"))
  ;[1 1 1] Stop colliding with enemy
  (if (== (`GameplayStatics.GetObjectClass` OtherActor) "/Game/TopDownBP/Blueprints/TopDownCharacter.TopDownCharacter_C")
    (set `self.CollidingEnemy` null)))

(event `self.ReceiveTick`
  (params (DeltaSeconds :type "Float (single-precision)")))

(event `self.TheOwner.OnDestroyed`
  ;[1 1 1] Cancel attack if owner gets killed.
  (`self.K2_DestroyActor`))

(fn `UserConstructionScript`)